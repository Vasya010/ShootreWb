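; Multiplayer game mode that respawns players as BP_Char_Master characters at randomly chosen Player Starts.
; On BeginPlay it caches all PlayerStart actors in a SpawnPoints array.
; Server_RespawnPlayer takes a controller, always spawns a new character regardless of collision using randomly indexed spawn point transforms, then has the controller possess it.
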(event `self.ReceiveBeginPlay`
  ;[1 1 1] Random Player Respawn (Replicated)
  (bind _outactors (`GameplayStatics.GetAllActorsOfClass` "/Script/Engine.PlayerStart"))
  (set `self.SpawnPoints` _outactors))

(event `Server_RespawnPlayer`
  (params (PlayerController :type "PlayerController Object Reference"))
  (bind _spawnpoints (`self.SpawnPoints`))
  (bind (_returnvalue_location _returnvalue_rotation) (`KismetMathLibrary.BreakTransform` (`self.GetTransform` (`|GetArrayItem` _spawnpoints (`KismetMathLibrary.RandomIntegerInRange` 0 (- (`KismetArrayLibrary.Array_Length` _spawnpoints) 1))))))
  ;[1 1 1] Random Player Respawn (Replicated)
  (`/Engine/EditorBlueprintResources/StandardMacros.IsValid` PlayerController
    (:`Is Valid`
      (bind _returnvalue (`|SpawnActorFromClass` "/Game/Asttes/Blueprints/Player/BP_Char_Master.BP_Char_Master_C" (`KismetMathLibrary.MakeTransform` _returnvalue_location _returnvalue_rotation) "AlwaysSpawn" "OverrideRootScale" null null))
      (`/Engine/EditorBlueprintResources/StandardMacros.IsValid` _returnvalue
        (:`Is Valid`
          (`Controller.Possess` PlayerController _returnvalue))))))

(fn `UserConstructionScript`)