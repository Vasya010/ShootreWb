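; Base projectile that covers bullets, explosives and bouncing projectiles, configured through bounce and explosive flags and a damage type.
; Non-bouncing hits play either surface-based impact effects or an explosion, while bouncing ones play bounce sounds and explode once movement stops.
; Both paths feed a shared damage step that rolls random damage, applying point damage with a headshot multiplier or full radial damage by damage type, then destroys the actor.
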(event `self.ReceiveBeginPlay`
  ;[0.8493 1 0] EventBeginPlay Set If Projectile Should Bounce
  (if (`self.IsShouldBounce?`)
    (set `ProjectileMovementComponent.bShouldBounce` true (`self.ProjectileMovement`))))

(event `self.ReceiveHit`
  (params (MyComp :type "PrimitiveComponent Object Reference") (Other :type "Actor Object Reference") (OtherComp :type "PrimitiveComponent Object Reference") (bSelfMoved :type Boolean) (HitLocation :type "Vector Structure") (HitNormal :type "Vector Structure") (NormalImpulse :type "Vector Structure") (Hit :type "HitResult Structure (by ref)"))
  (bind _returnvalue (`self.K2_GetActorLocation`))
  (bind (_bblockinghit _binitialoverlap _time _distance _location _impactpoint _normal _impactnormal _physmat _hitactor _hitcomponent _hitbonename) (`GameplayStatics.BreakHitResult` Hit))
  (bind _returnvalue_2 (`self.GetInstigatorController`))
  (bind _returnvalue_3 (`KismetMathLibrary.RandomIntegerInRange` (`self.MinDamage`) (`self.MaxDamage`)))
  (bind _returnvalue_4 (`KismetMathLibrary.Conv_IntToDouble` _returnvalue_3))
  ;[1 1 1] On Event Hit Check If Should Bounce Or If Is Explosive If Not Play Impact Sound & Particle Effect
  (if (not (`self.IsShouldBounce?`))
    (if (not (`self.IsExplosive?`))
      (`GameplayStatics.PlaySoundAtLocation` (select `EPhysicalSurface` (`PhysicalMaterial.SurfaceType` _physmat) :`SurfaceType_Default` (`self.DefaultBulletImpactSound`) :`SurfaceType1` (`self.CharacterBulletImpactSound`) :!type "SoundBase Object Reference") HitLocation (struct) 1.0 1.0 0.0 null null null null)
      (`GameplayStatics.SpawnEmitterAtLocation` (select `EPhysicalSurface` (`PhysicalMaterial.SurfaceType` _physmat) :`SurfaceType_Default` (`self.DefaultBulletImpactPS`) :`SurfaceType1` (`self.CharacterBulletImpactPS`)) HitLocation (`KismetMathLibrary.MakeRotFromZ` HitNormal))
      (else
        ;[1 1 1] On Projectile Stop Moving This Is To Make The Project Explode/PlaySound/Deal Damage When It Stops
        (`GameplayStatics.PlaySoundAtLocation` (`self.ExplosionSound`) _returnvalue (struct) 1.0 1.0 0.0 null null null null :!label _label)
        (`GameplayStatics.SpawnEmitterAtLocation` (`self.ExplosionPS`) _returnvalue (`KismetMathLibrary.MakeRotFromZ` HitNormal))))
    ;[1 1 1] Deal Damage Includes Critical Damage & Random Damage
    (switch `/Game/Asttes/Blueprints/Weapons/Masters/E_DamageTypes` (`self.DamageType`)
      (:`NewEnumerator1`
        (switch `name` _hitbonename
          (:`Default`
            (`GameplayStatics.ApplyDamage` _hitactor _returnvalue_4 _returnvalue_2 self "/Script/Engine.DamageType"))
          (:`head`
            (`GameplayStatics.ApplyDamage` _hitactor (`KismetMathLibrary.Conv_IntToDouble` (* _returnvalue_3 (`self.CriticalDamageMultiplier`))) _returnvalue_2 self "/Script/Engine.DamageType"))))
      (:`NewEnumerator2`
        (`GameplayStatics.ApplyRadialDamage` :`BaseDamage` _returnvalue_4 :`Origin` (`self.K2_GetActorLocation`) :`DamageRadius` (`self.DamageRadius`) :`DamageTypeClass` "/Script/Engine.DamageType" :`DamageCauser` self :`InstigatedByController` _returnvalue_2 :`bDoFullDamage` true)))
    (`self.K2_DestroyActor`)))

(event `self.ProjectileMovement.OnProjectileStop`
  (params (ImpactResult :type "HitResult Structure (by ref)"))
  ;[1 1 1] On Projectile Stop Moving This Is To Make The Project Explode/PlaySound/Deal Damage When It Stops
  (if (`self.IsShouldBounce?`)
    (goto _label)))

(event `self.ProjectileMovement.OnProjectileBounce`
  (params (ImpactResult :type "HitResult Structure (by ref)") (ImpactVelocity :type "Vector Structure (by ref)"))
  ;[1 1 1] Play Sound When Projectile Is Set To Bounce
  (if (`self.IsShouldBounce?`)
    (`GameplayStatics.PlaySoundAtLocation` (`self.BounceSound`) (`self.K2_GetActorLocation`) (struct) 1.0 1.0 0.0 null null null null)))

(fn `UserConstructionScript`)