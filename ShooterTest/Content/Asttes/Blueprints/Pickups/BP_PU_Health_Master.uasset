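; Master Blueprint for a health pickup that heals an overlapping player character and respawns after a delay.
; Overlap calls a server event that, below max health, multicasts the pickup sound, adds clamped health, then hides the actor and disables collision until the respawn timer ends.
; Floating text shows the heal amount and yaws each tick toward player 0's follow camera.
; The icon-spin timeline is never triggered.
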(event `self.ReceiveBeginPlay`
  ;[1 1 1] Creates Floating Text of "HealthAmountToGivePlayer" Above Pickup - Always Faces Camera
  (`TextRenderComponent.K2_SetText` (`self.TextRender`) (`KismetTextLibrary.Conv_IntToText` (`self.HealthAmountToGivePlayer`))))

(event `self.ReceiveTick`
  (params (DeltaSeconds :type "Float (single-precision)"))
  (bind _textrender (`self.TextRender`))
  ;[1 1 1] Creates Floating Text of "HealthAmountToGivePlayer" Above Pickup - Always Faces Camera
  (bind _asbp_char_master (cast `/Game/Asttes/Blueprints/Player/BP_Char_Master` (`GameplayStatics.GetPlayerPawn` 0)))
  (`/Engine/EditorBlueprintResources/StandardMacros.IsValid` _asbp_char_master
    (:`Is Valid`
      (`SceneComponent.K2_SetWorldRotation` _textrender (`KismetMathLibrary.MakeRotator` 0.0 0.0 (.yaw (`KismetMathLibrary.FindLookAtRotation` (`SceneComponent.K2_GetComponentLocation` _textrender) (`SceneComponent.K2_GetComponentLocation` (`/Game/Asttes/Blueprints/Player/BP_Char_Master.FollowCam` _asbp_char_master))))) false false))))

(event `Multicast_PickupFX`
  (`GameplayStatics.PlaySoundAtLocation` (`self.PickupSound`) (`self.K2_GetActorLocation`) (struct) 1.0 1.0 0.0 null null null null))

(event `self.ReceiveActorBeginOverlap`
  (params (OtherActor :type "Actor Object Reference"))
  (bind _asbp_char_master (cast `/Game/Asttes/Blueprints/Player/BP_Char_Master` OtherActor))
  (`self.Server_GiveHealth` _asbp_char_master))

(event `Server_GiveHealth`
  (params (Player :type "/Game/Asttes/Blueprints/Player/BP_Char_Master Object Reference"))
  (bind _spherecollision (`self.SphereCollision`))
  (bind _currenthealth (`/Game/Asttes/Blueprints/Player/BP_Char_Master.CurrentHealth` Player))
  (bind _maxhealth (`/Game/Asttes/Blueprints/Player/BP_Char_Master.MaxHealth` Player))
  (if (< _currenthealth _maxhealth)
    (`self.Multicast_PickupFX`)
    (set `/Game/Asttes/Blueprints/Player/BP_Char_Master.CurrentHealth` (`KismetMathLibrary.Clamp` (+ _currenthealth (`self.HealthAmountToGivePlayer`)) 0 _maxhealth) Player)
    (`self.SetActorHiddenInGame` true)
    (`PrimitiveComponent.SetCollisionEnabled` _spherecollision "NoCollision")
    (`KismetSystemLibrary.Delay` (`self.RespawnTimer`))
    (`PrimitiveComponent.SetCollisionEnabled` _spherecollision "QueryOnly")
    (`self.SetActorHiddenInGame` false)))

(fn `UserConstructionScript`)