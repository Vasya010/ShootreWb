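; Moving platform that shuttles and rotates between its origin and a configurable end transform, reversing mid-travel when a BP_Char_Master overlaps its safety collider.
; Two timelines, rate-scaled by travel time, drive the relative location and rotation lerps.
; Each finished travel plays stop audio, waits StopDelay, then restarts motor sounds and runs the opposite direction.
; The construction script previews end or midpoint transforms through editor flags.
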(event `self.SafetyCollider.OnComponentBeginOverlap`
  (params (OverlappedComponent :type "PrimitiveComponent Object Reference") (OtherActor :type "Actor Object Reference") (OtherComp :type "PrimitiveComponent Object Reference") (OtherBodyIndex :type Integer) (bFromSweep :type Boolean) (SweepResult :type "HitResult Structure (by ref)"))
  (bind _platform_travel_timeline (`self.Platform Travel Timeline`))
  (bind _motorloop_02_cue (`self.MotorLoop_02_Cue`))
  ;[1 1 1] Reverses Direction if collision occurs with Actor
  (cast `/Game/Asttes/Blueprints/Player/BP_Char_Master` OtherActor)
  (if (`ActorComponent.IsActive` _platform_travel_timeline)
    (if (`TimelineComponent.IsReversing` _platform_travel_timeline)
      (`|ExecutionSequence`
        (:`then_0`
          ;[1 1 1] Sets End Location and Rotation- Stop Delay- Reversing
          (bind (_direction _platform_travel) (`Timeline|Platform Travel Timeline` :!label _label) ; Float Translation Curve
            (:`Update`
              (`SceneComponent.K2_SetRelativeLocation` (`self.Platform`) (`KismetMathLibrary.VLerp` (0.0 0.0 0.0) (`self.EndLocation`) _platform_travel) false false))
            (:`Finished`
              (`|ExecutionSequence`
                (:`then_0`
                  (`KismetSystemLibrary.Delay` (`self.StopDelay`))
                  (`|ExecutionSequence`
                    (:`then_0`
                      ;[1 1 1] Start/Stop Audio
                      (`AudioComponent.Play` (`self.Platform_Start_01_Cue`) 0.0))
                    (:`then_1`
                      (switch `ETimelineDirection` _direction
                        (:`Forward`
                          (`self.PlatformReverese`))
                        (:`Backward`
                          (`self.PlatformForward`)))
                      (`AudioComponent.Play` _motorloop_02_cue 0.0))))
                (:`then_1`
                  (`AudioComponent.Play` (`self.SteamStop_01_03_Cue`) 0.0)
                  (`AudioComponent.Stop` _motorloop_02_cue))))))
        (:`then_1`
          (bind (_direction_2 _platform_rotation) (`Timeline|Platform Rotation Timeline` :!label _label_2) ; Float Rotation Curve
            (:`Update`
              (`SceneComponent.K2_SetRelativeRotation` (`self.Platform`) (`KismetMathLibrary.MakeRotator` (.x (`KismetMathLibrary.VLerp` (0.0 0.0 0.0) (`self.EndRotation`) _platform_rotation)) (.y (`KismetMathLibrary.VLerp` (0.0 0.0 0.0) (`self.EndRotation`) _platform_rotation)) (.z (`KismetMathLibrary.VLerp` (0.0 0.0 0.0) (`self.EndRotation`) _platform_rotation))) false false)))))
      (else
        (`|ExecutionSequence`
          (:`then_0`
            (goto _label :!via `Reverse`))
          (:`then_1`
            (goto _label_2 :!via `Reverse`)))))))

(event `PlatformForward`
  ;[1 1 1] Sets End Location and Rotation- Stop Delay- Reversing
  ;;[1 1 1] Reverses Direction if collision occurs with Actor
  (`|ExecutionSequence`
    (:`then_0`
      (goto _label :!via `PlayFromStart`))
    (:`then_1`
      (goto _label_2 :!via `PlayFromStart`))))

(event `PlatformReverese`
  ;[1 1 1] Sets End Location and Rotation- Stop Delay- Reversing
  ;;[1 1 1] Reverses Direction if collision occurs with Actor
  (`|ExecutionSequence`
    (:`then_0`
      (goto _label :!via `ReverseFromEnd`))
    (:`then_1`
      (goto _label_2 :!via `ReverseFromEnd`))))

(event `self.ReceiveBeginPlay`
  (bind _returnvalue (/ 1.0 (`self.TravelTimeInSeconds`)))
  ;[1 1 1] Sets Travel and Rotation Speed
  (`TimelineComponent.SetPlayRate` (`self.Platform Travel Timeline`) _returnvalue)
  (`TimelineComponent.SetPlayRate` (`self.Platform Rotation Timeline`) _returnvalue)
  (set `self.EndLocationPreview` true) ; Safety to Defeat Test during Play
)

(fn `UserConstructionScript`
  (bind _endrotation (`self.EndRotation`))
  (bind _endlocationpreview (`self.EndLocationPreview`))
  (bind _endlocation (`self.EndLocation`))
  (`SceneComponent.K2_SetRelativeLocation` (`self.Platform`) (`KismetMathLibrary.SelectVector` (`KismetMathLibrary.SelectVector` (/ _endlocation 2) _endlocation (`self.MidPointPreview`)) (0.0 0.0 0.0) _endlocationpreview) false false)
  (`SceneComponent.K2_SetRelativeRotation` (`self.Platform`) (`KismetMathLibrary.MakeRotator` (.x (`KismetMathLibrary.SelectVector` (`KismetMathLibrary.SelectVector` (/ _endrotation 2) _endrotation (`self.MidPointPreview`)) (0.0 0.0 0.0) _endlocationpreview)) (.y (`KismetMathLibrary.SelectVector` (`KismetMathLibrary.SelectVector` (/ _endrotation 2) _endrotation (`self.MidPointPreview`)) (0.0 0.0 0.0) _endlocationpreview)) (.z (`KismetMathLibrary.SelectVector` (`KismetMathLibrary.SelectVector` (/ _endrotation 2) _endrotation (`self.MidPointPreview`)) (0.0 0.0 0.0) _endlocationpreview))) false false))