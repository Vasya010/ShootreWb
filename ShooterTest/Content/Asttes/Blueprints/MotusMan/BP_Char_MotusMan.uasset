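; BP_Char_MotusMan is a damageable MotusMan NPC that loops a demo animation and audio, dies at zero health, and respawns.
; AnyDamage clamps health and triggers a multicast kill event, which plays death sound and animation, then hides the actor and disables mesh collision.
; After a respawn delay it restores visibility, collision, loop and health.
; A DoOnce, reset on Tick while alive, prevents repeated death sequences.
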(event `self.ReceiveBeginPlay`
  ;[1 1 1] Nps
  (set `self.CurrentHealth` (`self.MaxHealth`))
  (`SkeletalMeshComponent.PlayAnimation` (`self.SkeletalMesh`) (`self.DemoAnimation`) true)
  (`AudioComponent.FadeIn` (`self.AudioLoop`) 0.1 1.0 0.0 "Linear"))

(event `self.ReceiveAnyDamage`
  (params (Damage :type "Float (single-precision)") (DamageType :type "DamageType Object Reference") (InstigatedBy :type "Controller Object Reference") (DamageCauser :type "Actor Object Reference"))
  ;[1 1 1] Nps
  (set `self.CurrentHealth` (`KismetMathLibrary.Clamp` (`KismetMathLibrary.FTrunc` (- (`KismetMathLibrary.Conv_IntToDouble` (`self.CurrentHealth`)) Damage)) 0 (`self.MaxHealth`)))
  (if (== (`self.CurrentHealth`) 0)
    (`self.Multicast_KillMotusMan`)))

(event `Multicast_KillMotusMan`
  ;[1 1 1] Nps
  (set `self.IsMotusManDead?` true)
  (`/Engine/EditorBlueprintResources/StandardMacros.DoOnce` false :!label _label
    (:`Completed`
      (`AudioComponent.FadeOut` (`self.AudioLoop`) 0.1 0.0 "Linear")
      (`GameplayStatics.SpawnSoundAttached` (`self.DeathSound`) (`self.SkeletalMesh`) "Neck1" (0.0 0.0 0.0) (struct) "KeepRelativeOffset" false 1.0 1.0 0.0 null null)
      (`SkeletalMeshComponent.PlayAnimation` (`self.SkeletalMesh`) (`self.DeathAnimation`) false)
      (`KismetSystemLibrary.Delay` 8.7)
      (`PrimitiveComponent.SetCollisionEnabled` (`self.SkeletalMesh`) "NoCollision")
      (`self.SetActorHiddenInGame` true)
      (`KismetSystemLibrary.Delay` (`self.RespawnRate`))
      (`PrimitiveComponent.SetCollisionEnabled` (`self.SkeletalMesh`) "QueryAndPhysics")
      (`self.SetActorHiddenInGame` false)
      (`AudioComponent.FadeIn` (`self.AudioLoop`) 0.1 1.0 0.0 "Linear")
      (`SkeletalMeshComponent.PlayAnimation` (`self.SkeletalMesh`) (`self.DemoAnimation`) true)
      (set `self.IsMotusManDead?` false)
      (set `self.CurrentHealth` (`self.MaxHealth`)))))

(event `self.ReceiveTick`
  (params (DeltaSeconds :type "Float (single-precision)"))
  ;[1 1 1] Nps
  (if (not (`self.IsMotusManDead?`))
    (goto _label :!via `Reset`)))

(fn `UserConstructionScript`)